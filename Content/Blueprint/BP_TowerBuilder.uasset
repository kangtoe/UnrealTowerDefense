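; Tower builder for a defense game, handling the build menu and entry to and exit from build mode.
; A tick after BeginPlay, it fills the game mode's tower UI wrap box with one button per data table row.
; OnBuildMode spawns the chosen tower class under the cursor as a preview.
; OffBuildMode resets that state but clears the preview reference before calling TogglePreview(false) on it.
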(event Custom|CreateBuildButtons
  (Widget|Panel|ClearChildren (Variables|Default|GetBuild%20Button%20Wrap%20Box))
  (bind _outrownames (DataTable|GetDataTableRowNames "/Game/Blueprint/Data/TowerBuildInfoDataTable.TowerBuildInfoDataTable"))
  (for _array_element _outrownames
    (bind _returnvalue (Utilities|GetDataTableRow "/Game/Blueprint/Data/TowerBuildInfoDataTable.TowerBuildInfoDataTable" _array_element)
      (:then
        (bind _returnvalue_2 (UserInterface|CreateWidget "/Game/Blueprint/UI/WBP_TowerBuildButton.WBP_TowerBuildButton_C"))
        (Default|InitButton _returnvalue_2 _returnvalue)
        (Widget|Panel|AddChild (Variables|Default|GetBuild%20Button%20Wrap%20Box) _returnvalue_2)))))

(event Custom|OnBuildMode
  (params (buildInfo :type Tower%20Build%20Info%20Struct%20Structure))
  (bind _returnvalue (Game|SpawnActorfromClass (.TowerClass (Utilities|Struct|BreakTowerBuildInfoStruct buildInfo)) (Math|Conversions|ToTransform(Vector) (.Location (CallFunction|GetLocationUnderCursor self))) "AlwaysSpawn" "MultiplyWithRoot" 0 0))
  (bind _output_get (Variables|Default|SetBuildTowerPreview _returnvalue))
  (Default|TogglePreview _output_get true)
  (Variables|Default|SetbBuildMode true))

(event Custom|OffBuildMode
  (bind _output_get (Variables|Default|SetBuildTowerPreview 0))
  (Default|TogglePreview _output_get false)
  (Variables|Default|SetBuildTowerPreview 0)
  (Variables|Default|SetbBuildMode false))

(event EventBeginPlay
  (Utilities|FlowControl|DelayUntilNextTick)
  (Utilities|FlowControl|Sequence
    (:then_0
      (bind _asbp_defense_game_mode_game (Utilities|Casting|CastToBP_DefenseGameModeGame (Game|GetGameMode)))
      (Variables|Default|SetBuild%20Button%20Wrap%20Box (Variables|/Game/Blueprint/UI/WBP_TowerUI.WBP_TowerUI_C|GetBuildButtonWrapBox (Variables|/Game/Blueprint/BP_DefenseGameModeGame.BP_DefenseGameModeGame_C|GetWBP_TowerUI _asbp_defense_game_mode_game))))
    (:then_1
      (CallFunction|CreateBuildButtons))))

(fn ConstructionScript)