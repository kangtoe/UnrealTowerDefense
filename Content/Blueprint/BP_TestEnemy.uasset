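; BP_TestEnemy is a test enemy that travels along the BP_SplinePath spline to its end and back, escaping by destroying itself at the start.
; Tick advances spline distance and flips direction at the end, with a random lateral offset set at spawn.
; Damage calls SetHealth, whose body is empty; clamping and death sit in a separate CustomEvent, and health-bar code is disconnected.
; GetMoveProgress maps the round trip to 0–1.
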(event Custom|SetLocationOnSpline
  (bind _spline (Variables|Default|GetSpline))
  (bind _distalongspline (Variables|Move|GetdistAlongSpline))
  (bind _returnvalue (Spline|GetTransformatDistanceAlongSpline _spline _distalongspline "World" false))
  (Transformation|SetActorTransform (Math|Transform|MakeTransform (.location _returnvalue) (.rotation _returnvalue) "1.000000,1.000000,1.000000"))
  (Transformation|AddActorLocalOffset (Variables|Move|GetmoveDelta) false false))

(event Custom|OnTakeAnyDamage_이벤트
  (params (DamagedActor :type Actor%20Object%20Reference) (Damage :type Float%20%28single-precision%29) (DamageType :type Damage%20Type%20Object%20Reference) (InstigatedBy :type Controller%20Object%20Reference) (DamageCauser :type Actor%20Object%20Reference))
  (CallFunction|SetHealth (- (Variables|Health|GetcurrHealth) Damage)))

(event Custom|CustomEvent
  (params (newHealth :type Float%20%28double-precision%29))
  (Variables|Health|SetcurrHealth (Math|Float|Clamp(Float) newHealth 0.0 (Variables|Health|GetmaxHealth)))
  (Utilities|FlowControl|Sequence
    (:then_1
      (if (<= (Variables|Health|GetcurrHealth) 0.0)
        (CallFunction|OnDead)))))

(event Custom|EnemyEscape
  (Actor|DestroyActor))

(event Custom|OnDead
  (Actor|DestroyActor))

(event EventTick
  (params (DeltaSeconds :type Float%20%28single-precision%29))
  (Variables|Default|SetdeltaSec DeltaSeconds)
  (Utilities|FlowControl|Sequence
    (:then_0
      (Variables|Move|SetdistAlongSpline (+ (Variables|Move|GetdistAlongSpline) (* (Variables|Default|GetdeltaSec) (Variables|Move|GetmoveSpeed) (Variables|Move|GetmoveDir)))) ; 스플라인 상의 다음 위치 구하기
      (CallFunction|SetLocationonSpline))
    (:then_1
      (if (== (Variables|Move|GetmoveDir) 1) ; 진행방향이 정방향인가?
        (if (> (Variables|Move|GetdistAlongSpline) (Spline|GetSplineLength (Variables|Default|GetSpline))) ; 스플라인 끝까지 도달?
          (Utilities|FlowControl|DoOnce false
            (:Completed
              (Variables|Move|SetmoveDir -1)
              (Transformation|AddRelativeRotation (Variables|Default|GetSkeletalMesh) "0.000000,180.000000,0.000000" false false))))))
    (:then_2
      (if (== (Variables|Move|GetmoveDir) -1) ; 적 탈출 여부 검사
        (if (<= (Variables|Move|GetdistAlongSpline) 0.0)
          (CallFunction|EnemyEscape))))))

(event EventBeginPlay
  (Utilities|FlowControl|Sequence
    (:then_0
      (bind _returnvalue (Actor|GetActorOfClass "/Game/Blueprint/BP_SplinePath.BP_SplinePath_C"))
      (Variables|Default|SetSpline (Variables|/Game/Blueprint/BP_SplinePath.BP_SplinePath_C|GetSpline _returnvalue))
      (CallFunction|SetLocationonSpline))
    (:then_1
      (CallFunction|SetHealth (Variables|Health|GetmaxHealth)))
    (:then_2
      (Variables|Move|SetmoveDelta (Math|Vector|MakeVector 0.0 (Math|Random|RandomFloatinRange -5e+01 5e+01) 0.0)))
    (:then_3
      (EventDispatchers|AssignOnTakeAnyDamage (delegate Custom|OnTakeAnyDamage_이벤트)))))

(fn ConstructionScript)

(fn SetHealth
  (params (newHealth :type Float%20%28double-precision%29)))

(fn GetMoveProgress
  (LocalVariables|SetmaxDist (Spline|GetSplineLength (Variables|Default|GetSpline)))
  (switch int (Variables|Move|GetmoveDir)
    (:-1
      (return (+ (Utilities|Operators|Divide (- (LocalVariables|GetmaxDist) (Variables|Move|GetdistAlongSpline)) (LocalVariables|GetmaxDist) 2.0) 0.5)) ; 역방향 진행도 0.5~1
    )
    (:1
      (return (Utilities|Operators|Divide (Variables|Move|GetdistAlongSpline) (LocalVariables|GetmaxDist) 2.0)) ; 정방향 진행도: 최대 0.5
    )))