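; Tower defense turret prototype that automatically tracks and shoots BP_EnemyTest actors within an attack range sized by the construction script.
; Range entry, after a short delay, or the current target leaving triggers selection of the overlapping enemy with the greatest move progress.
; Tick smoothly rotates the head toward the target and drives a DoOnce-and-Delay cycle that spawns BP_Bullet at the arrow with the tower's damage.
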(event OnComponentBeginOverlap(AttackRangeSphere)
  (params (OverlappedComponent :type Primitive%20Component%20Object%20Reference) (OtherActor :type Actor%20Object%20Reference) (OtherComp :type Primitive%20Component%20Object%20Reference) (OtherBodyIndex :type Integer) (bFromSweep :type Boolean) (SweepResult :type Hit%20Result%20Structure%20%28by%20ref%29))
  (Utilities|FlowControl|Delay 0.1)
  (CallFunction|FindTarget))

(event Custom|FireBullet
  (bind _returnvalue (Game|SpawnActorfromClass "/Game/Blueprint/BP_Bullet.BP_Bullet_C" (Transformation|GetWorldTransform (Variables|Default|GetArrow)) "Undefined" "MultiplyWithRoot" 0 0))
  (Variables|/Game/Blueprint/BP_Bullet.BP_Bullet_C|Setdamage _returnvalue (Variables|Default|GetAttackDamage)))

(event Custom|LookTarget
  (bind _targetenemy (Variables|Targeting|GetTargetEnemy))
  (bind _towerhead (Variables|Default|GetTowerHead))
  (Utilities|IsValid _targetenemy
    (:Is%20Valid
      (Transformation|SetWorldRotation (Variables|Default|GetTowerHead) (Math|Rotator|Lerp(Rotator) (Transformation|GetWorldRotation _towerhead) (Math|Rotator|FindLookatRotation (Transformation|GetWorldLocation _towerhead) (Transformation|GetSocketLocation (Variables|/Game/Blueprint/BP_EnemyTest.BP_EnemyTest_C|GetCapsule _targetenemy) "None")) (* (Variables|Default|GetDelta%20Seconds) 1e+01) true) false false))))

(event Custom|CheckTargetInRanage
  (Utilities|IsValid (Variables|Targeting|GetTargetEnemy)
    (:Is%20Valid
      (if (not (Collision|IsOverlappingActor (Variables|Default|GetAttackRangeSphere) (Variables|Targeting|GetTargetEnemy) :!class /Script/Engine.PrimitiveComponent))
        (Variables|Targeting|SetTargetEnemy 0)
        (CallFunction|FindTarget)))))

(event Custom|FindTarget
  (for _array_element (Collision|GetOverlappingActors (Variables|Default|GetAttackRangeSphere) "/Game/Blueprint/BP_EnemyTest.BP_EnemyTest_C" :!class /Script/Engine.PrimitiveComponent)
    (bind _asbp_enemy_test (Utilities|Casting|CastToBP_EnemyTest _array_element))
    (bind _progress (Default|GetMoveProgress _asbp_enemy_test))
    (if (> _progress (Variables|Targeting|GetMoveProgressTmp))
      (Variables|Targeting|SetMoveProgressTmp _progress)
      (Variables|Targeting|SetTargetEnemy _asbp_enemy_test)))
  (Variables|Targeting|SetMoveProgressTmp 0.0))

(event Custom|FireCheck
  (Utilities|IsValid (Variables|Targeting|GetTargetEnemy)
    (:Is%20Valid
      (Utilities|FlowControl|DoOnce false :!label _label
        (:Completed
          (Utilities|FlowControl|Delay (Variables|Default|GetAttackInterval))
          (CallFunction|FireBullet)
          (goto _label Reset))))))

(event EventTick
  (params (DeltaSeconds :type Float%20%28single-precision%29))
  (Variables|Default|SetDelta%20Seconds DeltaSeconds)
  (Utilities|FlowControl|Sequence
    (:then_0
      (CallFunction|CheckTargetinRanage)
      (CallFunction|LookTarget)
      (CallFunction|FireCheck))))

(fn ConstructionScript
  (bind _attackrange (Variables|Default|GetAttackRange))
  (Transformation|SetWorldScale3D (Variables|Default|GetAttackRangeSphere) (Math|Conversions|ToVector(Float) _attackrange))
  (Components|Sphere|SetSphereRadius (Variables|Default|GetSphere) (* _attackrange 1e+02) true))