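; Tower selection manager that tracks which single tower is currently selected and keeps the tower info UI in sync with it.
; SelectTower clears the previous selection, toggles the new tower on, stores it as SelectedTower and passes it to SetTowerInfoUI.
; DeselectTower toggles off any valid selected tower, then always clears the reference and calls SetTowerInfoUI with no tower.
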(event Custom|SelectTower
  (params (NewSelectedTower :type BP%20Tower%20Test%20Object%20Reference))
  (CallFunction|DeselectTower)
  (Default|ToggleSelect NewSelectedTower true)
  (bind _output_get (Variables|Default|SetSelectedTower NewSelectedTower))
  (CallFunction|SetTowerInfoUI _output_get))

(event Custom|DeselectTower
  (Utilities|FlowControl|Sequence
    (:then_0
      (Utilities|IsValid (Variables|Default|GetSelectedTower)
        (:Is%20Valid
          (Default|ToggleSelect (Variables|Default|GetSelectedTower) false))))
    (:then_1
      (Variables|Default|SetSelectedTower 0)
      (CallFunction|SetTowerInfoUI))))

(fn ConstructionScript)