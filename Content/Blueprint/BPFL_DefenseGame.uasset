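; Blueprint function library of shared helpers for a tower defense game.
; Gold, tower selector, tower builder and tower UI helpers reach their targets by casting the game mode to BP_DefenseGameModeGame.
; Cursor helpers trace from player 0 to find a tower, a world location or an actor's distance from that location.
; The tower info panel shows level and a name found by matching the tower's class against data table rows.
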(fn TryAdjustGold
  (params (bForcePay :type Boolean) (Amount :type Integer) (WorldContextObject :type Object%20Object%20Reference))
  (LocalVariables|SetForcePay bForcePay)
  (LocalVariables|Setm_Amount Amount)
  (bind _asbp_defense_game_mode_game (Utilities|Casting|CastToBP_DefenseGameModeGame (Game|GetGameMode WorldContextObject)))
  (bind (_fail _consume) (Default|TryAdjustGold (Variables|/Game/Blueprint/BP_DefenseGameModeGame.BP_DefenseGameModeGame_C|GetBP_GoldManager _asbp_defense_game_mode_game) (LocalVariables|GetForcePay) (LocalVariables|Getm_Amount)))
  (return _fail _consume))

(fn GetTowerUnderCursor
  (params (WorldContextObject :type Object%20Object%20Reference))
  (bind _asbp_tower_test_base (Utilities|Casting|CastToBP_TowerTestBase (.HitActor (Collision|BreakHitResult (.HitResult (Game|Player|GetHitResultUnderCursorbyChannel (Game|GetPlayerController WorldContextObject) "TraceTypeQuery1" true)))))
    (:then
      (return _asbp_tower_test_base))
    (:CastFailed
      (return 0))))

(fn GetTowerSelector
  (params (WorldContextObject :type Object%20Object%20Reference))
  (bind _asbp_defense_game_mode_game (Utilities|Casting|CastToBP_DefenseGameModeGame (Game|GetGameMode WorldContextObject)))
  (return (Variables|/Game/Blueprint/BP_DefenseGameModeGame.BP_DefenseGameModeGame_C|GetBP_TowerSelector _asbp_defense_game_mode_game)))

(fn GetTowerBuilder
  (params (WorldContextObject :type Object%20Object%20Reference))
  (bind _asbp_defense_game_mode_game (Utilities|Casting|CastToBP_DefenseGameModeGame (Game|GetGameMode WorldContextObject)))
  (return (Variables|/Game/Blueprint/BP_DefenseGameModeGame.BP_DefenseGameModeGame_C|GetBP_TowerBuilder _asbp_defense_game_mode_game)))

(fn SetTowerInfoUI
  (params (Tower :type BP%20Tower%20Test%20Base%20Object%20Reference))
  (LocalVariables|Setm_Tower Tower)
  (Utilities|FlowControl|Sequence
    (:then_0
      (bind _asbp_defense_game_mode_game (Utilities|Casting|CastToBP_DefenseGameModeGame (Game|GetGameMode)))
      (LocalVariables|SetTowerInfoCanvas (Variables|/Game/Blueprint/UI/WBP_TowerUI.WBP_TowerUI_C|GetTowerInfoCanvasPanel (Variables|/Game/Blueprint/BP_DefenseGameModeGame.BP_DefenseGameModeGame_C|GetWBP_TowerUI _asbp_defense_game_mode_game)))
      (LocalVariables|SetTowerNameText (Variables|/Game/Blueprint/UI/WBP_TowerUI.WBP_TowerUI_C|GetTowerNameText (Variables|/Game/Blueprint/BP_DefenseGameModeGame.BP_DefenseGameModeGame_C|GetWBP_TowerUI _asbp_defense_game_mode_game)))
      (LocalVariables|SetTowerLevelText (Variables|/Game/Blueprint/UI/WBP_TowerUI.WBP_TowerUI_C|GetTowerLevelText (Variables|/Game/Blueprint/BP_DefenseGameModeGame.BP_DefenseGameModeGame_C|GetWBP_TowerUI _asbp_defense_game_mode_game))))
    (:then_1
      (Utilities|IsValid (LocalVariables|Getm_Tower) ; 오브젝트가 유효하지 않는 경우 초기화
        (:Is%20Valid
          (Widget|SetVisibility (LocalVariables|GetTowerInfoCanvas) "Visible"))
        (:Is%20Not%20Valid
          (Widget|SetVisibility (LocalVariables|GetTowerInfoCanvas) "Hidden")
          (return))))
    (:then_2
      (LocalVariables|SetTowerBuildInfo (CallFunction|GetTowerBuildInfo (Utilities|GetClass (LocalVariables|Getm_Tower)) (LocalVariables|Getm_Tower))))
    (:then_3
      (Rendering|Components|TextRender|SetText (LocalVariables|GetTowerNameText) (Utilities|Text|ToText(String) (.TowerName (Utilities|Struct|BreakTowerBuildInfoStruct (LocalVariables|GetTowerBuildInfo))))))
    (:then_4
      (Rendering|Components|TextRender|SetText (LocalVariables|GetTowerLevelText) (Utilities|Text|ToText(Integer) (Variables|/Game/Blueprint/Towers/BP_TowerTestBase.BP_TowerTestBase_C|GetTowerLevel (LocalVariables|Getm_Tower)))))))

(fn GetTowerBuildInfo
  (params (TowerClass :type BP%20Tower%20Test%20Base%20Class%20Reference))
  (LocalVariables|Setm_TowerClass TowerClass)
  (bind _outrownames (DataTable|GetDataTableRowNames "/Game/Blueprint/Data/TowerBuildInfoDataTable.TowerBuildInfoDataTable"))
  (for _array_element _outrownames
    (bind _returnvalue (Utilities|GetDataTableRow "/Game/Blueprint/Data/TowerBuildInfoDataTable.TowerBuildInfoDataTable" _array_element)
      (:then
        (if (== (.TowerClass (Utilities|Struct|BreakTowerBuildInfoStruct _returnvalue)) (LocalVariables|Getm_TowerClass))
          (return _returnvalue))))))

(fn GetLocationUnderCursor
  (params (WorldContextObject :type Object%20Object%20Reference))
  (bind _returnvalue (Game|GetPlayerController WorldContextObject))
  (bind (_hitresult _returnvalue_2) (Game|Player|GetHitResultUnderCursorbyChannel _returnvalue "TraceTypeQuery3" true))
  (if _returnvalue_2
    (return (.Location (Collision|BreakHitResult _hitresult)) true)
    (else
      (return "0, 0, 0" false))))

(fn ToggleBuildCancelUI
  (params (toggle :type Boolean))
  (bind _asbp_defense_game_mode_game (Utilities|Casting|CastToBP_DefenseGameModeGame (Game|GetGameMode)))
  (Default|ToggleBuildCancelUI (Variables|/Game/Blueprint/BP_DefenseGameModeGame.BP_DefenseGameModeGame_C|GetWBP_TowerUI _asbp_defense_game_mode_game) toggle))

(fn GetDistfromCursor
  (params (타깃 :type Actor%20Object%20Reference))
  (return (Math|Vector|Distance(Vector) (.Location (CallFunction|GetLocationUnderCursor 타깃 타깃)) (Transformation|GetActorLocation 타깃))))