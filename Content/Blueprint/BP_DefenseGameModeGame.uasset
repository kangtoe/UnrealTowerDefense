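; Game mode for a tower defense game that sets up the core gameplay actors and UI when play begins.
; A BeginPlay sequence spawns the enemy spawner, gold manager, tower selector and tower builder at its own transform, then creates the tower UI widget and adds it to the viewport.
; It keeps references to each, except the tower builder, whose variable is set to None instead of the spawned actor.
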(event EventBeginPlay
  (Utilities|FlowControl|Sequence
    (:then_0
      (bind _returnvalue (Game|SpawnActorfromClass "/Game/Blueprint/BP_EnemySpawner.BP_EnemySpawner_C" (Transformation|GetActorTransform) "Undefined" "MultiplyWithRoot" 0 0))
      (Variables|Default|SetBP_EnemySpawner _returnvalue))
    (:then_1
      (bind _returnvalue_2 (Game|SpawnActorfromClass "/Game/Blueprint/BP_GoldManager.BP_GoldManager_C" (Transformation|GetActorTransform) "Undefined" "MultiplyWithRoot" 0 0))
      (Variables|Default|SetBP_GoldManager _returnvalue_2))
    (:then_2
      (bind _returnvalue_3 (Game|SpawnActorfromClass "/Game/Blueprint/BP_TowerSelector.BP_TowerSelector_C" (Transformation|GetActorTransform) "Undefined" "MultiplyWithRoot" 0 0))
      (Variables|Default|SetBP_TowerSelector _returnvalue_3))
    (:then_3
      (Game|SpawnActorfromClass "/Game/Blueprint/BP_TowerBuilder.BP_TowerBuilder_C" (Transformation|GetActorTransform) "Undefined" "MultiplyWithRoot" 0 0)
      (Variables|Default|SetBP_TowerBuilder 0))
    (:then_4
      (bind _returnvalue_4 (UserInterface|CreateWidget "/Game/Blueprint/UI/WBP_TowerUI.WBP_TowerUI_C"))
      (UserInterface|Viewport|AddtoViewport _returnvalue_4 0)
      (Variables|Default|SetWBP_TowerUI _returnvalue_4))))

(fn ConstructionScript)