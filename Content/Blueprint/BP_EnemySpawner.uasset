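; BP_EnemySpawner is an actor that spawns a series of BP_EnemyTest enemies at its own transform, starting on BeginPlay.
; A self-calling SpawnEnemyLoop event spawns one enemy, decrements SpawnCountLeft, then waits SpawnDelay before repeating while the count stays above zero.
; The first enemy appears immediately, because spawning happens before the count check.
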(event Custom|SpawnEnemy
  (Game|SpawnActorfromClass "/Game/Blueprint/BP_EnemyTest.BP_EnemyTest_C" (Transformation|GetActorTransform) "Undefined" "MultiplyWithRoot" 0 0))

(event Custom|SpawnEnemyLoop
  (CallFunction|SpawnEnemy)
  (bind _result (Math|Integer|DecrementInt (Variables|Default|GetSpawnCountLeft))
    (:%20%20
      (if (> _result 0)
        (Utilities|FlowControl|Delay (Variables|Default|GetSpawnDelay))
        (CallFunction|SpawnEnemyLoop) ; 재귀적 호출
      ))))

(event EventBeginPlay
  (CallFunction|SpawnEnemyLoop))

(fn ConstructionScript)