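; Base tower-defense tower, with cursor-following placement preview, selection highlight, and gold-based upgrading and selling.
; Outside preview, Tick keeps a target in the range sphere, choosing the enemy with most path progress, and lerps the head toward it.
; A forward sphere trace gates interval-limited BP_Bullet shots carrying damage, debuff, gold and area data.
; Upgrades expand range and recompute upgrade and sell costs; the max-level check is a constant true.
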(event OnComponentBeginOverlap(Sphere)
  (params (OverlappedComponent :type Primitive%20Component%20Object%20Reference) (OtherActor :type Actor%20Object%20Reference) (OtherComp :type Primitive%20Component%20Object%20Reference) (OtherBodyIndex :type Integer) (bFromSweep :type Boolean) (SweepResult :type Hit%20Result%20Structure%20%28by%20ref%29))
  (Utilities|FlowControl|Delay 0.1)
  (CallFunction|FindTarget))

(event Custom|FireBullet
  (bind _returnvalue (Game|SpawnActorfromClass "/Game/Blueprint/BP_Bullet.BP_Bullet_C" (Transformation|GetWorldTransform (Variables|Default|GetArrow)) "AlwaysSpawn" "MultiplyWithRoot" 0 0))
  (Default|InitBullet _returnvalue (Variables|Attacking|GetDefaultAttackDamage) (Variables|Debuff|GetDebuff%20Info) (Variables|Attacking|GetHit%20Gold) (Variables|Attacking|GetAttackAreaRadius)))

(event Custom|LookTarget
  (bind _targetenemy (Variables|Targeting|GetTargetEnemy))
  (bind _towerhead (Variables|Default|GetTowerHead))
  (Utilities|IsValid _targetenemy
    (:Is%20Valid
      (Transformation|SetWorldRotation (Variables|Default|GetTowerHead) (Math|Rotator|Lerp(Rotator) (Transformation|GetWorldRotation _towerhead) (Math|Rotator|FindLookatRotation (Transformation|GetWorldLocation _towerhead) (Transformation|GetSocketLocation (Variables|/Game/Blueprint/BP_EnemyTest.BP_EnemyTest_C|GetCapsule _targetenemy) "None")) (* (Variables|Default|GetDelta%20Seconds) 1e+01) true) false false))))

(event Custom|TryLevelUp
  (if true ; 최대 레벨 도달 전인가?
    (bind _fail (CallFunction|TryAdjustGold false (* (Variables|Default|GetUpgradeCost) -1) self))
    (if (not _fail) ; 골드 충분?
      (Math|Integer|IncrementInt (Variables|Default|GetTowerLevel)
        (:%20%20
          (CallFunction|SetAttackRange (* (Variables|Attacking|GetDefaultAttackRange) (+ (* (Variables|Default|GetTowerLevel) 0.2) 1.0)))
          (CallFunction|UpdateUpgradeCost)
          (CallFunction|SetTowerInfoUI self))))))

(event Custom|CkeckTargetInRange
  (if (not (CallFunction|CheckEnemyinRange (Variables|Targeting|GetTargetEnemy)))
    (Variables|Targeting|SetTargetEnemy 0)
    (CallFunction|FindTarget)))

(event Custom|SetAttackRange
  (params (range :type Float%20%28double-precision%29))
  (bind _output_get (Variables|Attacking|SetCurrAttackRange range))
  (Transformation|SetWorldScale3D (Variables|Default|GetAttackRangeIndicator) (Math|Vector|MakeVector (* _output_get 0.01) (* _output_get 0.01) 0.01))
  (Components|Sphere|SetSphereRadius (Variables|Default|GetSphere) _output_get true))

(event Custom|SellTower
  (bind _self self)
  (bind _bp_towerselector (CallFunction|GetTowerSelector _self))
  (Utilities|FlowControl|Sequence
    (:then_0
      (if (== (Variables|/Game/Blueprint/BP_TowerSelector.BP_TowerSelector_C|GetSelectedTower _bp_towerselector) _self)
        (Default|DeselectTower _bp_towerselector)))
    (:then_1
      (Variables|/Game/Blueprint/BP_TowerBuildPoint.BP_TowerBuildPoint_C|SetbTowerBuilded (Variables|Default|GetBuildPoint) false))
    (:then_2
      (CallFunction|TryAdjustGold false (Variables|Default|GetSellCost) self)
      (Actor|DestroyActor))))

(event Custom|SetBuildPoint
  (params (BuildPoint :type BP%20Tower%20Build%20Point%20Object%20Reference))
  (bind _output_get (Variables|Default|SetBuildPoint BuildPoint))
  (Variables|/Game/Blueprint/BP_TowerBuildPoint.BP_TowerBuildPoint_C|SetbTowerBuilded _output_get true))

(event Custom|UpdateUpgradeCost
  (Variables|Default|SetUpgradeCost (+ (Variables|Default|GetBuildCost) (* (Variables|Default|GetTowerLevel) (Variables|Default|GetUpgradeCost))))
  (Variables|Default|SetSellCost (/ (+ (Variables|Default|GetBuildCost) (Variables|Default|GetUpgradeCost)) 2)))

(event Custom|FindTarget
  (for _array_element (Collision|GetOverlappingActors (Variables|Default|GetSphere) "/Game/Blueprint/BP_EnemyTest.BP_EnemyTest_C" :!class /Script/Engine.PrimitiveComponent)
    (bind _asbp_enemy_test (Utilities|Casting|CastToBP_EnemyTest _array_element))
    (bind _progress (Default|GetMoveProgress _asbp_enemy_test))
    (if (> _progress (Variables|Targeting|GetfMoveProgress))
      (Variables|Targeting|SetfMoveProgress _progress)
      (Variables|Targeting|SetTargetEnemy _asbp_enemy_test)))
  (Variables|Targeting|SetfMoveProgress 0.0))

(event Custom|FireCheck
  (if (Variables|Attacking|GetEnemyOnSight)
    (Utilities|FlowControl|DoOnce false :!label _label
      (:Completed
        (CallFunction|FireBullet)
        (Utilities|FlowControl|Delay (Variables|Attacking|GetAttackInterval))
        (goto _label Reset)))))

(event Custom|CheckEnemyOnSight
  (bind _arrow (Variables|Default|GetArrow))
  (bind _returnvalue (Transformation|GetWorldLocation _arrow))
  (Variables|Attacking|SetEnemyOnSight false)
  (bind _outhits (Collision|MultiSphereTraceByChannel _returnvalue (+ _returnvalue (* (Math|Vector|GetForwardVector _arrow) (* (Variables|Attacking|GetCurrAttackRange) 0.5))) 1e+01 "TraceTypeQuery1" false 0 "None"))
  (bind _array_element (Utilities|Array|ForEachLoopwithBreak _outhits :!label _label)
    (:LoopBody
      (bind _asbp_enemy_test (Utilities|Casting|CastToBP_EnemyTest (.HitActor (Collision|BreakHitResult _array_element))))
      (if (CallFunction|CheckEnemyinRange _asbp_enemy_test)
        (Variables|Attacking|SetEnemyOnSight true)
        (goto _label Break)))))

(event Custom|ToggleSelect
  (params (toggle :type Boolean))
  (Development|SetHiddeninGame (Variables|Default|GetAttackRangeIndicator) (not toggle) false)
  (if toggle
    (Rendering|Material|SetOverlayMaterial (Variables|Default|GetTowerHead) "/Game/M_Overlay.M_Overlay" :!class /Script/Engine.MeshComponent)
    (else
      (Rendering|Material|SetOverlayMaterial (Variables|Default|GetTowerHead) 0 :!class /Script/Engine.MeshComponent))))

(event Custom|TogglePreview
  (params (Toggle :type Boolean))
  (bind _output_get (Variables|Preview|SetbPreviewMod Toggle))
  (if _output_get
    (CallFunction|SetTowerMaterials (Variables|프리뷰|GetPreviewMaterial))
    (else
      (CallFunction|SetTowerMaterials (Variables|프리뷰|GetNomalMaterial)))))

(event Custom|SetTowerMaterials
  (params (Material :type Material%20Interface%20Object%20Reference))
  (Rendering|Material|SetMaterial (Variables|Default|GetTowerBody) 0 Material)
  (Rendering|Material|SetMaterial (Variables|Default|GetCube) 0 Material)
  (Rendering|Material|SetMaterial (Variables|Default|GetTowerHead) 0 Material))

(event Custom|FollowCursor
  (Transformation|SetActorLocation (.Location (CallFunction|GetLocationUnderCursor self)) false false))

(event EventBeginPlay
  (Variables|Default|SetBuildCost (.BuildCost (Utilities|Struct|BreakTowerBuildInfoStruct (CallFunction|GetTowerBuildInfo (Utilities|GetClass self)))))
  (CallFunction|UpdateUpgradeCost))

(event EventTick
  (params (DeltaSeconds :type Float%20%28single-precision%29))
  (Variables|Default|SetDelta%20Seconds DeltaSeconds)
  (if (not (Variables|Preview|GetbPreviewMod))
    (CallFunction|CkeckTargetinRange)
    (CallFunction|LookTarget)
    (CallFunction|CheckEnemyonSight)
    (CallFunction|FireCheck)))

(fn ConstructionScript
  (CallFunction|SetAttackRange (Variables|Attacking|GetDefaultAttackRange))
  (CallFunction|ToggleSelect false)
  (CallFunction|TogglePreview false))

(fn CheckEnemyinRange
  (params (TargetEnemy :type BP%20Enemy%20Test%20Object%20Reference))
  (Utilities|IsValid TargetEnemy
    (:Is%20Valid
      (if (Collision|IsOverlappingActor (Variables|Default|GetSphere) TargetEnemy :!class /Script/Engine.PrimitiveComponent)
        (return true)
        (else
          _)))
    (:Is%20Not%20Valid
      _))
  (return false))