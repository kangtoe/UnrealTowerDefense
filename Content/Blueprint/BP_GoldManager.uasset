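; Gold manager Blueprint that holds the gold balance and puts the gold display and tower build button widgets on screen at BeginPlay.
; TryAdjustGold applies a signed amount and refreshes the text, with ForcePay clamping shortfalls to zero.
; An unforced shortfall leaves gold unchanged, shows a not-enough-gold widget and returns true, while successful adjustments return false.
; UpdateGoldText reuses TryAdjustGold with a zero amount to refresh the display.
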(event Custom|UpdateGoldText
  (CallFunction|TryAdjustGold false))

(event EventBeginPlay
  (bind _returnvalue (UserInterface|CreateWidget "/Game/Blueprint/UI/WBP_Gold.WBP_Gold_C"))
  (bind _output_get (Variables|Default|SetWBP_Gold _returnvalue))
  (UserInterface|Viewport|AddtoViewport _output_get 0)
  (CallFunction|UpdateGoldText)
  (bind _returnvalue_2 (UserInterface|CreateWidget "/Game/Blueprint/UI/WBP_TowerBuildButton.WBP_TowerBuildButton_C"))
  (UserInterface|Viewport|AddtoViewport _returnvalue_2 0))

(fn ConstructionScript)

(fn TryAdjustGold
  (params (bForcePay :type Boolean) (Amount :type Integer))
  (LocalVariables|SetForcePay bForcePay)
  (bind _output_get (LocalVariables|SetResultGold (+ (Variables|Default|GetGold) Amount)))
  (if (>= _output_get 0) ; 지불할 골드가 충분한가?
    (Variables|Default|SetGold (LocalVariables|GetResultGold))
    (elif (LocalVariables|GetForcePay) ; 골드가 부족해도 진행되어야 하는가?
      (Variables|Default|SetGold 0)
      (else
        (bind _returnvalue (UserInterface|CreateWidget "/Game/Blueprint/UI/WBP_NotEnoughGold.WBP_NotEnoughGold_C"))
        (UserInterface|Viewport|AddtoViewport _returnvalue 0)
        (return true))))
  (Rendering|Components|TextRender|SetText (Variables|/Game/Blueprint/UI/WBP_Gold.WBP_Gold_C|GetGoldText (Variables|Default|GetWBP_Gold)) (Utilities|Text|ToText(Integer) (Variables|Default|GetGold)))
  (return false))