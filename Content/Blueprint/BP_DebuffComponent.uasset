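; Timed debuff component that slows the BP_EnemyTest that owns it, with Frozen as the only handled effect.
; BeginPlay caches the enemy and scales its move speed down by the DebuffAmount percentage.
; Tick counts down LeftDebuffTime, then OnEndDebuff applies the inverse multiplier to undo the slow and destroys the component.
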(event Custom|OnEndDebuff
  (Utilities|FlowControl|Sequence
    (:then_0
      (switch Utilities|FlowControl|Switch|SwitchonDebuffType "NewEnumerator0"
        (:NewEnumerator0
          (Default|AdjustMoveSpeed (Variables|Default|GetBP%20Enemy) (/ 1e+02 (- 1e+02 (Variables|Default|GetDebuffAmount)))))))
    (:then_1
      (Components|DestroyComponent))))

(event EventBeginPlay
  (bind _asbp_enemy_test (Utilities|Casting|CastToBP_EnemyTest (Components|GetOwner)))
  (Variables|Default|SetBP%20Enemy _asbp_enemy_test)
  (switch Utilities|FlowControl|Switch|SwitchonDebuffType "NewEnumerator0"
    (:NewEnumerator0
      (Default|AdjustMoveSpeed (Variables|Default|GetBP%20Enemy) (/ (- 1e+02 (Variables|Default|GetDebuffAmount)) 1e+02)))))

(event EventTick
  (params (DeltaSeconds :type Float%20%28single-precision%29))
  (bind _output_get (Variables|Default|SetLeftDebuffTime (- (Variables|Default|GetLeftDebuffTime) DeltaSeconds)))
  (if (<= _output_get 0.0)
    (CallFunction|OnEndDebuff)))