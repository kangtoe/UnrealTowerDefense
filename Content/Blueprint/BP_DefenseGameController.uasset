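; BP_DefenseGameController is a controller that drives the camera pawn through Enhanced Input.
; BeginPlay adds the IMC_Camera mapping context to the local player's input subsystem.
; Move and rotate actions apply speed-scaled local offsets and yaw directly to player pawn 0, without sweep or delta-time scaling.
; The zoom action casts that pawn to BP_CamPawn and passes the scaled input to its AdjustZoom.
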(event Input|EnhancedActionEvents|EnhancedInputActionIA_Move
  (params (ActionValue :type Vector%202D%20Structure) (ElapsedSeconds :type Float%20%28double-precision%29) (TriggeredSeconds :type Float%20%28double-precision%29) (InputAction :type Input%20Action%20Object%20Reference :default "/Game/Input/IA_Move.IA_Move"))
  (:Triggered
    (Transformation|AddActorLocalOffset (Game|Player|GetPlayerPawn 0) (Math|Conversions|ToVector(Vector2D) (* ActionValue (Variables|Default|GetMoveSpeed))) false false)))

(event Input|EnhancedActionEvents|EnhancedInputActionIA_Rotate
  (params (ActionValue :type Float%20%28double-precision%29) (ElapsedSeconds :type Float%20%28double-precision%29) (TriggeredSeconds :type Float%20%28double-precision%29) (InputAction :type Input%20Action%20Object%20Reference :default "/Game/Input/IA_Rotate.IA_Rotate"))
  (:Triggered
    (Transformation|AddActorLocalRotation (Game|Player|GetPlayerPawn 0) (Math|Rotator|MakeRotator 0.0 0.0 (* ActionValue (Variables|Default|GetRotateSpeed))) false false)))

(event Input|EnhancedActionEvents|EnhancedInputActionIA_Zoom
  (params (ActionValue :type Float%20%28double-precision%29) (ElapsedSeconds :type Float%20%28double-precision%29) (TriggeredSeconds :type Float%20%28double-precision%29) (InputAction :type Input%20Action%20Object%20Reference :default "/Game/Input/IA_Zoom.IA_Zoom"))
  (:Triggered
    (bind _asbp_cam_pawn (Utilities|Casting|CastToBP_CamPawn (Game|Player|GetPlayerPawn 0)))
    (Default|AdjustZoom _asbp_cam_pawn (* ActionValue (Variables|Default|GetZoomSpeed)))))

(event EventBeginPlay
  (bind _returnvalue (PlayerController|LocalPlayerSubsystems|GetEnhancedInputLocalPlayerSubsystem))
  ;[0.05098 0.05098 0.05098] Add Mapping Context
  (Utilities|IsValid _returnvalue
    (:Is%20Valid
      (Input|AddMappingContext _returnvalue "/Game/Input/IMC_Camera.IMC_Camera" 0 "(bIgnoreAllPressedKeysUntilRelease=True,bForceImmediately=False)"))))

(fn ConstructionScript)