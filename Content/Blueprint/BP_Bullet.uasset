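; BP_Bullet is a tower-fired projectile that damages the BP_EnemyTest actor it hits.
; InitBullet receives the damage value, and the Sphere's begin overlap applies it to the enemy, then destroys the bullet.
; An overlap that fires before initialization waits one tick so the damage value can be set first.
; OnDestroy, also triggered when the lifetime delay ends, spawns an explosion emitter and removes the actor.
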(event OnComponentBeginOverlap(Sphere)
  (params (OverlappedComponent :type Primitive%20Component%20Object%20Reference) (OtherActor :type Actor%20Object%20Reference) (OtherComp :type Primitive%20Component%20Object%20Reference) (OtherBodyIndex :type Integer) (bFromSweep :type Boolean) (SweepResult :type Hit%20Result%20Structure%20%28by%20ref%29))
  (bind _output_get (Variables|Default|SetOther%20Actor OtherActor))
  (if (Variables|Default|GetbInit) ; 생성한 타워로부터 초기화 되지 않은 경우, 다음 프레임(초기화 이후)에 타격 처리
    _
    (else
      (Utilities|FlowControl|DelayUntilNextTick)))
  (bind _asbp_enemy_test (Utilities|Casting|CastToBP_EnemyTest _output_get))
  (Game|Damage|ApplyDamage _asbp_enemy_test (Variables|Default|Getdamage) 0 self)
  (CallFunction|OnDestroy))

(event Custom|OnDestroy
  (bind _sphere (Variables|Default|GetSphere))
  (bind _returnvalue (Transformation|GetWorldTransform _sphere))
  (Effects|SpawnEmitteratLocation "/Game/StarterContent/Particles/P_Explosion.P_Explosion" (.location _returnvalue) (.rotation _returnvalue))
  (Actor|DestroyActor))

(event Custom|InitBullet
  (params (Damage :type Float%20%28double-precision%29))
  (Variables|Default|Setdamage Damage)
  (Variables|Default|SetbInit true))

(event EventBeginPlay
  (Utilities|FlowControl|Delay (Variables|Default|GetliveTime))
  (CallFunction|OnDestroy))

(fn ConstructionScript)